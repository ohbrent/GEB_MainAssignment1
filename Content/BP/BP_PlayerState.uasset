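; Player state Blueprint that times a run, with a start countdown and a time limit that leads to failure.
; Tick lowers StartTimer until it drops below zero, then sets RunStart, which lets RunTimer accumulate until RunEnd is set.
; Once RunTimer reaches EndTime, it sets RunEnd and calls OnFailed, which repeats every tick while that condition holds.
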(event EventBeginPlay)

(event EventTick
  (params (DeltaSeconds :type Float%20%28single-precision%29))
  (Utilities|FlowControl|Sequence
    (:then_0
      (if (>= (Variables|Default|GetStartTimer) 0.0)
        (Variables|Default|SetStartTimer (- (Variables|Default|GetStartTimer) DeltaSeconds))
        (else
          (Variables|Default|SetRunStart true))))
    (:then_1
      (if (and (Variables|Default|GetRunStart) (not (Variables|Default|GetRunEnd)))
        (Variables|Default|SetRunTimer (+ (Variables|Default|GetRunTimer) DeltaSeconds))))
    (:then_2
      (if (>= (Variables|Default|GetRunTimer) (Variables|Default|GetEndTime))
        (Variables|Default|SetRunEnd true)
        (Default|CallOnFailed)))))

(fn ConstructionScript)