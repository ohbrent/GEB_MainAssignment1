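; BP_RunPowerUp is a pickup that unlocks running for the player.
; A cube spins every tick until BP_ThirdPersonCharacter overlaps the sphere.
; The overlap tints the Niagara particles translucent green and destroys the cube, light and sphere, leaving the actor in place.
; It then sets CanRun on the BP_PlayerState cached from player index 0 at BeginPlay and calls CallOnRunActivate on it.
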(event OnComponentBeginOverlap(Sphere)
  (params (OverlappedComponent :type Primitive%20Component%20Object%20Reference) (OtherActor :type Actor%20Object%20Reference) (OtherComp :type Primitive%20Component%20Object%20Reference) (OtherBodyIndex :type Integer) (bFromSweep :type Boolean) (SweepResult :type Hit%20Result%20Structure%20%28by%20ref%29))
  (bind _as_bp_player_state (Variables|Default|GetAs%20BP%20Player%20State))
  (Utilities|Casting|CastToBP_ThirdPersonCharacter OtherActor)
  (Niagara|SetNiagaraVariable(LinearColor) (Variables|Default|GetNiagara) "ParticleColor" (Math|Color|MakeColor 0.0 1.0 0.0 0.3))
  (Components|DestroyComponent (Variables|Default|GetCube))
  (Components|DestroyComponent (Variables|Default|GetPointLight))
  (Components|DestroyComponent (Variables|Default|GetSphere))
  (Variables|/Game/BP/BP_PlayerState.BP_PlayerState_C|SetCanRun _as_bp_player_state true)
  (Default|CallOnRunActivate _as_bp_player_state))

(event EventBeginPlay
  (bind _asbp_player_state (Utilities|Casting|CastToBP_PlayerState (Game|GetPlayerState 0)))
  (Variables|Default|SetAs%20BP%20Player%20State _asbp_player_state))

(event EventTick
  (params (DeltaSeconds :type Float%20%28single-precision%29))
  (bind _cube (Variables|Default|GetCube))
  (Utilities|IsValid _cube
    (:Is%20Valid
      (Transformation|AddWorldRotation _cube (Math|Rotator|MakeRotator 1.0 1.0 1.0) false false))))

(fn ConstructionScript)