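; BP_SpawnObjectTrigger is a trigger volume that enables falling-object spawning when the player character walks into it.
; On BeginPlay it caches the first player's BP_PlayerState and tints its Niagara particles red.
; When a BP_ThirdPersonCharacter overlaps the Box, it turns the particles green and sets SpawnFallingObject on that player state.
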(event OnComponentBeginOverlap(Box)
  (params (OverlappedComponent :type Primitive%20Component%20Object%20Reference) (OtherActor :type Actor%20Object%20Reference) (OtherComp :type Primitive%20Component%20Object%20Reference) (OtherBodyIndex :type Integer) (bFromSweep :type Boolean) (SweepResult :type Hit%20Result%20Structure%20%28by%20ref%29))
  (Utilities|Casting|CastToBP_ThirdPersonCharacter OtherActor)
  (Niagara|SetNiagaraVariable(LinearColor) (Variables|Default|GetNiagara) "ParticleColor" (Math|Color|MakeColor 0.0 1.0 0.0))
  (Variables|/Game/BP/BP_PlayerState.BP_PlayerState_C|SetSpawnFallingObject (Variables|Default|GetAs%20BP%20Player%20State) true))

(event EventBeginPlay
  (bind _asbp_player_state (Utilities|Casting|CastToBP_PlayerState (Game|GetPlayerState 0)))
  (Variables|Default|SetAs%20BP%20Player%20State _asbp_player_state)
  (Niagara|SetNiagaraVariable(LinearColor) (Variables|Default|GetNiagara) "ParticleColor" (Math|Color|MakeColor 1.0 0.0 0.0)))

(fn ConstructionScript)