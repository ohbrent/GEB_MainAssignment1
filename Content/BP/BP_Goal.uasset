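; Goal actor that marks when the player character reaches it.
; On BeginPlay it caches the first player's BP_PlayerState.
; When a BP_ThirdPersonCharacter enters its Box, it turns the Niagara particles and point light green, then fires the OnGoal dispatcher on that cached player state.
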(event OnComponentBeginOverlap(Box)
  (params (OverlappedComponent :type Primitive%20Component%20Object%20Reference) (OtherActor :type Actor%20Object%20Reference) (OtherComp :type Primitive%20Component%20Object%20Reference) (OtherBodyIndex :type Integer) (bFromSweep :type Boolean) (SweepResult :type Hit%20Result%20Structure%20%28by%20ref%29))
  (bind _returnvalue (Math|Color|MakeColor 0.0 1.0 0.0 0.3))
  (Utilities|Casting|CastToBP_ThirdPersonCharacter OtherActor)
  (Niagara|SetNiagaraVariable(LinearColor) (Variables|Default|GetNiagara) "ParticleColor" _returnvalue)
  (Rendering|Components|Light|SetLightColor (Variables|Default|GetPointLight) _returnvalue true)
  (Default|CallOnGoal (Variables|Default|GetAs%20BP%20Player%20State)))

(event EventBeginPlay
  (bind _asbp_player_state (Utilities|Casting|CastToBP_PlayerState (Game|GetPlayerState 0)))
  (Variables|Default|SetAs%20BP%20Player%20State _asbp_player_state))

(fn ConstructionScript)