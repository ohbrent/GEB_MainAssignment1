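; BP_Spawner is an actor that spawns a row of falling objects when the player state signals it.
; It caches BP_PlayerState on BeginPlay and polls its SpawnFallingObject flag every Tick.
; Once the flag is set, it spawns five BP_SpawnObject actors evenly spaced along world Y from its root, randomly setting some meshes to unit scale, then destroys itself, making it one-shot.
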(event EventBeginPlay
  (bind _asbp_player_state (Utilities|Casting|CastToBP_PlayerState (Game|GetPlayerState 0)))
  (Variables|Default|SetAs%20BP%20Player%20State _asbp_player_state))

(event EventTick
  (params (DeltaSeconds :type Float%20%28single-precision%29))
  (if (Variables|/Game/BP/BP_PlayerState.BP_PlayerState_C|GetSpawnFallingObject (Variables|Default|GetAs%20BP%20Player%20State))
    (for _index (range 0 4)
      (bind _returnvalue (Game|SpawnActorfromClass "/Game/BP/BP_SpawnObject.BP_SpawnObject_C" (Math|Transform|MakeTransform (+ (Transformation|GetWorldLocation (Variables|Default|GetDefaultSceneRoot)) (Math|Vector|MakeVector 0.0 (* _index 400) 0.0)) "0, 0, 0" "1.000000,1.000000,1.000000") "Undefined" "MultiplyWithRoot" 0 0))
      (if (Math|Random|RandomBool)
        (Transformation|SetWorldScale3D (Variables|/Game/BP/BP_SpawnObject.BP_SpawnObject_C|GetStaticMesh _returnvalue) "1.000000,1.000000,1.000000")))
    (Actor|DestroyActor)))

(fn ConstructionScript)