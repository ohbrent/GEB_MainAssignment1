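; BP_Canon is a cannon actor that automatically fires projectiles at a fixed interval.
; Tick accumulates delta time in ShootTimer and resets it whenever it reaches ShootPeriod.
; Each shot spawns a BP_Shootable at the root component's transform and launches its Sphere with a strong physics impulse along the root's forward vector.
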(event EventBeginPlay)

(event Collision|EventActorBeginOverlap
  (params (OtherActor :type Actor%20Object%20Reference)))

(event EventTick
  (params (DeltaSeconds :type Float%20%28single-precision%29))
  (bind _defaultsceneroot (Variables|Default|GetDefaultSceneRoot))
  (bind _returnvalue (Transformation|GetWorldTransform _defaultsceneroot))
  (bind _output_get (Variables|Default|SetShootTimer (+ DeltaSeconds (Variables|Default|GetShootTimer))))
  (if (>= _output_get (Variables|Default|GetShootPeriod))
    (Variables|Default|SetShootTimer 0.0)
    (bind _returnvalue_2 (Game|SpawnActorfromClass "/Game/BP/BP_Shootable.BP_Shootable_C" (Math|Transform|MakeTransform (.location _returnvalue) (.rotation _returnvalue) (.scale _returnvalue)) "Undefined" "MultiplyWithRoot" 0 0))
    (Physics|AddImpulse (Variables|/Game/BP/BP_Shootable.BP_Shootable_C|GetSphere _returnvalue_2) (* (Math|Rotator|GetRotationXVector (.rotation _returnvalue)) "100000.000000,100000.000000,100000.000000") "None" false)))

(fn ConstructionScript)