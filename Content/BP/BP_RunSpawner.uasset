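; Trigger actor that spawns a timed wave of BP_SpawnObject actors around the running player.
; Box overlap by the third-person character turns the Niagara ParticleColor green and starts spawning, while actor overlap caches the player reference.
; Tick accumulates a timer, placing each enlarged object at a fixed world-space offset from the player with random X spread.
; Spawning stops after eight objects, and the count is never reset.
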(event OnComponentBeginOverlap(Box)
  (params (OverlappedComponent :type Primitive%20Component%20Object%20Reference) (OtherActor :type Actor%20Object%20Reference) (OtherComp :type Primitive%20Component%20Object%20Reference) (OtherBodyIndex :type Integer) (bFromSweep :type Boolean) (SweepResult :type Hit%20Result%20Structure%20%28by%20ref%29))
  (Utilities|Casting|CastToBP_ThirdPersonCharacter OtherActor)
  (Niagara|SetNiagaraVariable(LinearColor) (Variables|Default|GetNiagara) "ParticleColor" (Class|KismetMathLibrary|LinearColorGreen))
  (Variables|Default|SetStart%20Spawn true))

(event EventBeginPlay)

(event Collision|EventActorBeginOverlap
  (params (OtherActor :type Actor%20Object%20Reference))
  (bind _asbp_third_person_character (Utilities|Casting|CastToBP_ThirdPersonCharacter (Game|Player|GetPlayerPawn 0)))
  (Variables|Default|SetAs%20BP%20Third%20Person%20Character _asbp_third_person_character))

(event EventTick
  (params (DeltaSeconds :type Float%20%28single-precision%29))
  (if (Variables|Default|GetStart%20Spawn)
    (Variables|Default|SetSpawnTimer (+ (Variables|Default|GetSpawnTimer) DeltaSeconds))
    (if (>= (Variables|Default|GetSpawnTimer) 1.2)
      (Variables|Default|SetSpawnTimer 0.0)
      (Game|SpawnActorfromClass "/Game/BP/BP_SpawnObject.BP_SpawnObject_C" (Math|Transform|MakeTransform (+ (Transformation|GetWorldLocation (Variables|/Script/Engine.Character|GetCapsuleComponent (Variables|Default|GetAs%20BP%20Third%20Person%20Character))) (Math|Vector|MakeVector (Math|Random|RandomFloatinRange -4e+02 4e+02) 1.2e+03 3e+02)) "0, 0, 0" "4.000000,4.000000,4.000000") "Undefined" "MultiplyWithRoot" 0 0)
      (bind _result (Math|Integer|IncrementInt (Variables|Default|GetSpawnCount))
        (:%20%20
          (if (>= _result 8)
            (Variables|Default|SetStart%20Spawn false)))))))

(fn ConstructionScript)